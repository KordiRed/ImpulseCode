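; Base gun actor for the player, providing firing, aim-down-sights, reload and ammo tracking.
; ADS blends the view target to the gun and back to its parent actor, syncing the player camera to control rotation while aimed.
; Fire spawns projectiles within a random cone, tighter in ADS, with camera shake and low-ammo audio; recoil and fire-rate helpers are separate.
; Reload waits out an arms montage, then refills from reserve ammo.
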(event Custom|FireGun
  ;[1 1 1] Fire
  (Variables|State|SetShoot? true))

(event Custom|StopFireGun
  ;[1 1 1] Fire
  (Variables|State|SetShoot? false))

(event Custom|Start%20ADS
  ;[1 1 1] ADS
  (Variables|State|SetADS? true)
  (Utilities|FlowControl|Delay 0.1)
  (Game|Player|SetViewTargetwithBlend (Game|GetPlayerController 0) self 0.2 "VTBlend_Linear" 0.0 false)
  (Audio|Components|Audio|Play (Variables|Default|GetScope_in) 0.0))

(event Custom|Stop%20ADS
  ;[1 1 1] ADS
  (Variables|State|SetADS? false)
  (Game|Player|SetViewTargetwithBlend (Game|GetPlayerController 0) (Actor|GetParentActor) 0.2 "VTBlend_Linear" 0.0 false)
  (Audio|Components|Audio|Play (Variables|Default|GetScope_out) 0.0))

(event Custom|Reload
  ;[1 1 1] Reload
  (if (and (!= (Variables|Ammo|GetClipSize) (Variables|Ammo|GetAmmoCurrent)) (> (Variables|Ammo|GetAmmoMax) 0))
    (Variables|State|SetReload? true)
    (bind _returnvalue (Animation|Montage|MontagePlay (Components|SkeletalMesh|GetAnimInstance (Variables|/Game/Blueprints/Player/BP_Player.BP_Player_C|GetArms (Variables|Default|GetBP_Player))) (Variables|SettingUpShots|GetReloadMontage) 1.0 "MontageLength" 0.0 true))
    (Utilities|FlowControl|Delay _returnvalue)
    (bind _output_get (Variables|Ammo|SetBulletDifference (- (Variables|Ammo|GetClipSize) (Variables|Ammo|GetAmmoCurrent))))
    (if (>= (Variables|Ammo|GetAmmoMax) _output_get)
      (Variables|Ammo|SetAmmoCurrent (Variables|Ammo|GetClipSize))
      (Variables|Ammo|SetAmmoMax (- (Variables|Ammo|GetAmmoMax) (Variables|Ammo|GetBulletDifference)))
      (else
        (Variables|Ammo|SetAmmoCurrent (+ (Variables|Ammo|GetAmmoCurrent) (Variables|Ammo|GetAmmoMax)))
        (Variables|Ammo|SetAmmoMax 0)))
    (Variables|State|SetReload? false)))

(event EventBeginPlay
  ;[1 1 1] Begin Play
  (bind _asbp_player (Utilities|Casting|CastToBP_Player (Game|GetPlayerCharacter 0)))
  (Variables|Default|SetBP_Player _asbp_player))

(event EventTick
  (params (DeltaSeconds :type Float%20%28single-precision%29))
  ;[1 1 1] ADS
  (if (Variables|State|GetADS?)
    (Transformation|SetWorldRotation (Variables|/Game/Blueprints/Player/BP_Player.BP_Player_C|GetCamera (Variables|Default|GetBP_Player)) (Pawn|GetControlRotation (Game|GetPlayerController 0) :!class /Script/Engine.Controller) false false)))

(fn ConstructionScript
  (|CallParentFunction))

(fn SprayAngle
  (params (MuzzleDirection :type Vector) (MaxAngle :type Float%20%28single-precision%29))
  (return (Math|Rotator|MakeRotfromX (Math|Random|RandomUnitVectorinConeinDegrees MuzzleDirection MaxAngle))))

(fn GetDelayfromFireRate
  (return (/ 0.6 (/ (Variables|Settingupshots|GetFireRate) 6e+01))))

(fn Recoil(PitchYaw)
  (params (Pitch :type Float%20%28single-precision%29) (Yaw :type Float%20%28single-precision%29))
  (bind _returnvalue (Game|GetPlayerController 0))
  (Class|PlayerController|AddPitchInput _returnvalue Pitch)
  (Class|PlayerController|AddYawInput _returnvalue Yaw))

(fn Fire
  (bind _arrow (Variables|Default|GetArrow))
  (bind _returnvalue (Transformation|GetWorldRotation _arrow))
  (bind _returnvalue_2 (Math|Vector|GetForwardVector _returnvalue))
  (if (Variables|State|GetShoot?)
    (if (not (Variables|State|GetReload?))
      (if (Variables|State|GetADS?)
        (LocalVariables|SetDirection (CallFunction|SprayAngle _returnvalue_2 (/ (Variables|SettingUpShots|GetMaxAngle) 5.4)))
        (else
          (LocalVariables|SetDirection (CallFunction|SprayAngle _returnvalue_2 (Variables|SettingUpShots|GetMaxAngle)))))
      (Game|SpawnActorfromClass "/Game/Blueprints/Weapon/Guns/BP_Projectile.BP_Projectile_C" (Math|Transform|MakeTransform (Transformation|GetWorldLocation (Variables|Default|GetArrow)) (LocalVariables|GetDirection) "1,1,1") "Undefined" 0 0)
      (Game|Feedback|ClientStartCameraShake (Game|GetPlayerController 0) "/Game/Blueprints/Weapon/Guns/BP_CameraShake.BP_CameraShake_C" 1.0 "CameraLocal" "0, 0, 0")
      (if (> (Variables|Ammo|GetAmmoCurrent) (/ (Variables|Ammo|GetClipSize) 3))
        (Audio|Components|Audio|Play (Variables|Default|GetShoot_full) 0.0)
        (else
          (Audio|Components|Audio|Play (Variables|Default|GetShoot_low) 0.0)))
      (Math|Integer|DecrementInt (Variables|Ammo|GetAmmoCurrent)
        (:%20%20
          (return))))))

(fn GetReloadState
  (return (Variables|State|GetReload?)))

(fn GetShootState
  (return (Variables|State|GetShoot?)))