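; BP_GunHammervolt is the Hammervolt gun Blueprint, adding automatic fire and recoil on top of its parent gun logic.
; After a brief delay, firing loops at the fire-rate delay while ammo and shoot state allow, playing the fire animation each shot.
; A recoil timeline drives pitch and yaw as it plays forward, counting recoil steps.
; Stopping or emptying reverses it at double speed, resetting the count and adding extra-pitch correction after longer bursts.
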(event EventStartADS
  (|CallParentFunction))

(event EventStopADS
  (|CallParentFunction))

(event EventTick
  (params (DeltaSeconds :type Float%20%28single-precision%29))
  (|CallParentFunction DeltaSeconds))

(event EventReload
  (|CallParentFunction))

(event EventStopFireGun
  (|CallParentFunction)
  (Components|Timeline|SetPlayRate (Variables|Default|GetRecoilTimeline) 2.0 :!label _label)
  (bind (_direction _pitch _yaw) (Timeline|RecoilTimeline Reverse)
    (:Update
      (switch Utilities|FlowControl|Switch|SwitchonETimelineDirection _direction
        (:Forward
          (CallFunction|Recoil(PitchYaw) _pitch _yaw)
          (Math|Float|IncrementFloat (Variables|Default|GetRecoil)
            (:%20%20
              (Utilities|FlowControl|Delay (CallFunction|GetDelayfromFireRate))
              (if (and (> (Variables|Default|GetAmmoCurrent) 0) (CallFunction|GetShootState))
                (CallFunction|Fire)
                (Components|Animation|PlayAnimation (Variables|Default|GetGun) "/Game/WeaponsMeshes/Hammervolt/Animations/Hammervolt_Fire_Anim.Hammervolt_Fire_Anim" false)
                (if (!= (Variables|Default|GetAmmoCurrent) 0)
                  (Components|Timeline|SetPlayRate (Variables|Default|GetRecoilTimeline) 1.0)
                  (Timeline|RecoilTimeline Play)
                  (else
                    (goto _label)))))))
        (:Backward
          (if (> (Variables|Default|GetRecoil) 7.0)
            (CallFunction|Recoil(PitchYaw) (+ _pitch 1.0) _yaw)
            (Variables|Default|SetRecoil 0.0)
            (else
              (Variables|Default|SetRecoil 0.0))))))))

(event EventFireGun
  (|CallParentFunction)
  (Utilities|FlowControl|Delay 0.1)
  (if (and (> (Variables|Default|GetAmmoCurrent) 0) (CallFunction|GetShootState)) :!label _label
    (CallFunction|Fire)
    (Components|Animation|PlayAnimation (Variables|Default|GetGun) "/Game/WeaponsMeshes/Hammervolt/Animations/Hammervolt_Fire_Anim.Hammervolt_Fire_Anim" false)
    (if (!= (Variables|Default|GetAmmoCurrent) 0)
      (Components|Timeline|SetPlayRate (Variables|Default|GetRecoilTimeline) 1.0)
      (bind (_direction _pitch _yaw) (Timeline|RecoilTimeline Play)
        (:Update
          (switch Utilities|FlowControl|Switch|SwitchonETimelineDirection _direction
            (:Forward
              (CallFunction|Recoil(PitchYaw) _pitch _yaw)
              (Math|Float|IncrementFloat (Variables|Default|GetRecoil)
                (:%20%20
                  (Utilities|FlowControl|Delay (CallFunction|GetDelayfromFireRate))
                  (goto _label))))
            (:Backward
              (if (> (Variables|Default|GetRecoil) 7.0)
                (CallFunction|Recoil(PitchYaw) (+ _pitch 1.0) _yaw)
                (Variables|Default|SetRecoil 0.0)
                (else
                  (Variables|Default|SetRecoil 0.0)))))))
      (else
        (Components|Timeline|SetPlayRate (Variables|Default|GetRecoilTimeline) 2.0)
        (Timeline|RecoilTimeline Reverse)))))

(fn ConstructionScript
  (|CallParentFunction))