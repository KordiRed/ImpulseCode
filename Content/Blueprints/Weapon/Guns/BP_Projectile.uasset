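; BP_Projectile is a gun projectile that deals damage to actors its collision sphere overlaps.
; On overlap it prints the other actor's name and sends it TakeDamageMessage.
; The damage value comes from player 0's currently held BP_GunParent child actor, read at impact rather than stored on the projectile.
; Hit and actor overlap events are empty, and physics impulse logic is left disconnected.
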(event OnComponentBeginOverlap(SphereColision)
  (params (OverlappedComponent :type Primitive%20Component%20Object%20Reference) (OtherActor :type Actor%20Object%20Reference) (OtherComp :type Primitive%20Component%20Object%20Reference) (OtherBodyIndex :type Integer) (bFromSweep :type Boolean) (SweepResult :type Hit%20Result%20Structure%20%28by%20ref%29))
  (Development|PrintString (Utilities|GetDisplayName OtherActor))
  (Class|BPIDamage|TakeDamage(Message) OtherActor (Variables|/Game/Blueprints/Weapon/Guns/BP_GunParent.BP_GunParent_C|GetDamage (.AsBP%20Gun%20Parent (Utilities|Casting|CastToBP_GunParent (Variables|/Script/Engine.ChildActorComponent|GetChildActor (Variables|/Game/Blueprints/Player/BP_Player.BP_Player_C|GetGun (.AsBP%20Player (Utilities|Casting|CastToBP_Player (Game|GetPlayerCharacter 0))))))))))

(event Collision|EventActorBeginOverlap
  (params (OtherActor :type Actor%20Object%20Reference)))

(event Collision|EventHit
  (params (MyComp :type Primitive%20Component%20Object%20Reference) (Other :type Actor%20Object%20Reference) (OtherComp :type Primitive%20Component%20Object%20Reference) (bSelfMoved :type Boolean) (HitLocation :type Vector :default "0, 0, 0") (HitNormal :type Vector :default "0, 0, 0") (NormalImpulse :type Vector :default "0, 0, 0") (Hit :type Hit%20Result%20Structure%20%28by%20ref%29)))

(fn ConstructionScript
  (|CallParentFunction))