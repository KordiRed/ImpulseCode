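; Energy gun Blueprint that adds delayed, automatic fire on top of its parent gun class.
; FireGun calls the parent, waits through a short fixed delay, then repeatedly calls Fire while ammo remains and the shoot state is active.
; The loop is built from latent Delays, spacing shots by the interval derived from the fire rate.
; Stop fire, aim-down-sights, tick, reload and construction only forward to the parent.
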(event EventStartADS
  (|CallParentFunction))

(event EventStopADS
  (|CallParentFunction))

(event EventTick
  (params (DeltaSeconds :type Float%20%28single-precision%29))
  (|CallParentFunction DeltaSeconds))

(event EventReload
  (|CallParentFunction))

(event EventStopFireGun
  (|CallParentFunction))

(event EventFireGun
  (|CallParentFunction)
  (Utilities|FlowControl|Delay 0.25)
  (if (and (> (Variables|Default|GetAmmoCurrent) 0) (CallFunction|GetShootState)) :!label _label
    (CallFunction|Fire)
    (Utilities|FlowControl|Delay (CallFunction|GetDelayfromFireRate))
    (goto _label)))

(fn ConstructionScript
  (|CallParentFunction))