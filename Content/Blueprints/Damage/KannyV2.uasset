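; KannyV2 is a damageable character with a floating world-space health bar.
; On begin play it caches the KannyHP widget and the player's camera, then fills its health.
; Each tick updates the bar's percent from current health and rotates it to face the camera.
; Damage lowers health, and at zero it disables capsule collision, ragdolls the mesh and hides the bar.
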(event EventBeginPlay
  ;[1 1 1] Begin Play
  (bind _askanny_hp (Utilities|Casting|CastToKannyHP (UserInterface|GetUserWidgetObject (Variables|Default|GetHPBar))))
  (Variables|HP|SetKanny%20HP _askanny_hp)
  (bind _asbp_player (Utilities|Casting|CastToBP_Player (Game|GetPlayerCharacter 0)))
  (Variables|Default|SetPlayer%20Camera (Variables|/Game/Blueprints/Player/BP_Player.BP_Player_C|GetCamera _asbp_player))
  (Variables|HP|SetHP (Variables|HP|GetHPMax)))

(event EventTick
  (params (DeltaSeconds :type Float%20%28single-precision%29))
  (bind _hpbar (Variables|Default|GetHPBar))
  ;[1 1 1] HPBar
  (Utilities|FlowControl|Sequence
    (:then_0
      (Progress|SetPercent (Variables|/Game/Blueprints/Damage/KannyHP.KannyHP_C|GetProgressBar_31 (Variables|HP|GetKanny%20HP)) (Math|Float|NormalizetoRange (Variables|HP|GetHP) 0.0 (Variables|HP|GetHPMax))))
    (:then_1
      (Transformation|SetWorldRotation _hpbar (Math|Rotator|FindLookatRotation (Transformation|GetWorldLocation _hpbar) (Transformation|GetWorldLocation (Variables|Default|GetPlayer%20Camera))) false false))))

(event EventTakeDamage
  (params (Damage :type Float%20%28single-precision%29))
  ;[1 1 1] Take Damage
  (bind _output_get (Variables|HP|SetHP (- (Variables|HP|GetHP) Damage)))
  (if (<= _output_get 0.0)
    (Collision|SetCollisionEnabled (Variables|Collision|GetCapsuleComponent) "NoCollision")
    (Physics|SetSimulatePhysics (Variables|Character|GetMesh) true)
    (Rendering|SetVisibility (Variables|Default|GetHPBar) false false)))

(fn ConstructionScript)